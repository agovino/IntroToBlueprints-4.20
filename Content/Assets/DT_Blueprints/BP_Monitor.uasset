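; BP_Monitor is an interactable monitor that lets the player switch the alarm state of a referenced AlarmLight.
; Its TriggerVolume toggles the tooltip text and enables player 0's input when an overlap begins, then toggles the text again and disables input when it ends.
; While input is enabled, pressing F calls ChangeAlarmState on AlarmLight if that reference is valid.
; Neither overlap event filters which actor triggers it.
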(event `self.TriggerVolume.OnComponentBeginOverlap`
  (params (OverlappedComponent :type "PrimitiveComponent Object Reference") (OtherActor :type "Actor Object Reference") (OtherComp :type "PrimitiveComponent Object Reference") (OtherBodyIndex :type Integer) (bFromSweep :type Boolean) (SweepResult :type "HitResult Structure (by ref)"))
  (`SceneComponent.ToggleVisibility` (`self.ToolTipText`) false)
  (`self.EnableInput` (`GameplayStatics.GetPlayerController` 0)))

(event `self.TriggerVolume.OnComponentEndOverlap`
  (params (OverlappedComponent :type "PrimitiveComponent Object Reference") (OtherActor :type "Actor Object Reference") (OtherComp :type "PrimitiveComponent Object Reference") (OtherBodyIndex :type Integer))
  (`SceneComponent.ToggleVisibility` (`self.ToolTipText`) false)
  (`self.DisableInput` (`GameplayStatics.GetPlayerController` 0)))

(event `Key|F`
  (params (Key :type "Key Structure"))
  (:`Pressed`
    (`/Engine/EditorBlueprintResources/StandardMacros.IsValid` (`self.AlarmLight`)
      (:`Is Valid`
        (`/Game/Assets/DT_Blueprints/BP_AlarmLight.ChangeAlarmState` (`self.AlarmLight`))
        (`/Game/Assets/DT_Blueprints/BP_AlarmLight.ChangeAlarmState` (`self.AlarmLight`))))))

(fn `UserConstructionScript`)